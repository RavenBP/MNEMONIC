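; BP_Altar is an interactable altar that the player pays Mind Guardian currency to activate, which in turn activates its linked Barrier.
; A sphere overlap shows or clears the cost prompt, built in the construction script, through the game mode's PlayerStatWidget.
; On interaction it requires currency strictly above the cost, spends it and sets IsActivated, otherwise reporting insufficient funds or existing activation in the same widget.
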(event OnComponentBeginOverlap(Sphere)
  (params (OverlappedComponent :type Primitive%20Component%20Object%20Reference) (OtherActor :type Actor%20Object%20Reference) (OtherComp :type Primitive%20Component%20Object%20Reference) (OtherBodyIndex :type Integer) (bFromSweep :type Boolean) (SweepResult :type Hit%20Result%20Structure%20%28by%20ref%29))
  (Utilities|Casting|CastToFirstPersonCharacter OtherActor)
  (Development|PrintString "Overlapping Altar")
  (bind _ascustom_game_mode (Utilities|Casting|CastToCustomGameMode (Game|GetGameMode)))
  (Variables|/Game/Blueprints/Widgets/BP_PlayerStatsWidget.BP_PlayerStatsWidget_C|SetInteraction%20Text (Variables|/Game/Maps/CustomGameMode.CustomGameMode_C|GetPlayerStatWidget _ascustom_game_mode) (Variables|AltarInteraction|GetInteraction%20Text)))

(event OnComponentEndOverlap(Sphere)
  (params (OverlappedComponent :type Primitive%20Component%20Object%20Reference) (OtherActor :type Actor%20Object%20Reference) (OtherComp :type Primitive%20Component%20Object%20Reference) (OtherBodyIndex :type Integer))
  (Utilities|Casting|CastToFirstPersonCharacter OtherActor)
  (Variables|/Game/Blueprints/Widgets/BP_PlayerStatsWidget.BP_PlayerStatsWidget_C|SetInteraction%20Text (Variables|/Game/Maps/CustomGameMode.CustomGameMode_C|GetPlayerStatWidget (stale OnComponentBeginOverlap(Sphere) _ascustom_game_mode)) ""))

(event EventOnInteraction
  (params (Player :type Character%20Object%20Reference))
  (bind _asfirst_person_character (Utilities|Casting|CastToFirstPersonCharacter Player))
  (if (Variables|AltarInteraction|GetIsActivated)
    (CallFunction|PrintInteractionText "This Altar is activated" :!label _label)
    (elif (> (Variables|/Game/Blueprints/FirstPersonCharacter.FirstPersonCharacter_C|GetMindGuardianCurrency _asfirst_person_character) (Variables|AltarInteraction|GetMGC%20Cost))
      (Default|SpendCurrency _asfirst_person_character (Variables|AltarInteraction|GetMGC%20Cost))
      (Default|Activate (Variables|AltarInteraction|GetBarrier))
      (Variables|AltarInteraction|SetIsActivated true)
      (goto _label)
      (else
        (CallFunction|PrintInteractionText "You don't have enough MGC for this Altar")))))

(event EventBeginPlay)

(fn ConstructionScript
  (Variables|AltarInteraction|SetInteraction%20Text (Utilities|Text|ToText(String) (Utilities|String|Append "Activating this Altar costs " (Utilities|String|ToString(Integer) (Variables|AltarInteraction|GetMGC%20Cost)) " MGC"))))

(fn PrintInteractionText
  (params (InteractionText :type Text))
  (bind _ascustom_game_mode (Utilities|Casting|CastToCustomGameMode (Game|GetGameMode)))
  (Variables|/Game/Blueprints/Widgets/BP_PlayerStatsWidget.BP_PlayerStatsWidget_C|SetInteraction%20Text (Variables|/Game/Maps/CustomGameMode.CustomGameMode_C|GetPlayerStatWidget _ascustom_game_mode) InteractionText))