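; BP_EngramTouch is a touchable engram actor that responds when the FirstPersonCharacter hits its mesh.
; The construction script applies the configurable StaticMesh variable to TouchEngramMesh.
; Each character hit prints a debug "Hello"; if IsActivated is true, it also plays ActivatedSound at the actor and calls Deactivate.
; Deactivate clears the flag and applies ActivatedMaterial, so the sound and material change do not repeat.
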(event OnComponentHit(touchEngramMesh)
  (params (HitComponent :type Primitive%20Component%20Object%20Reference) (OtherActor :type Actor%20Object%20Reference) (OtherComp :type Primitive%20Component%20Object%20Reference) (NormalImpulse :type Vector :default "0, 0, 0") (Hit :type Hit%20Result%20Structure%20%28by%20ref%29))
  (Utilities|Casting|CastToFirstPersonCharacter OtherActor)
  (Development|PrintString "Hello")
  (if (Variables|Default|GetisActivated)
    (Audio|PlaySoundatLocation (Variables|Default|GetactivatedSound) (Transformation|GetActorLocation) "0, 0, 0" 1.0 1.0 0.0 0 0 0)
    (CallFunction|Deactivate)))

(event EventBeginPlay)

(event Collision|EventActorBeginOverlap
  (params (OtherActor :type Actor%20Object%20Reference)))

(fn ConstructionScript
  (Components|StaticMesh|SetStaticMesh (Variables|Default|GettouchEngramMesh) (Variables|Default|GetstaticMesh)))

(fn Deactivate
  (Variables|Default|SetisActivated false)
  (Rendering|Material|SetMaterial (Variables|Default|GettouchEngramMesh) 0 (Variables|Default|GetactivatedMaterial))
  (return))