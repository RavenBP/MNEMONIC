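; BP_NarrativeTrigger is a one-shot box trigger that plays character dialogue with subtitles when the FirstPersonCharacter enters it.
; On overlap it disables box collision, plays the audio on the character's dialogue sound component and shows the speaker and line on the player HUD.
; After a delay matching the audio's duration it hides the subtitles and destroys itself.
; The construction script sizes the box from an extent variable.
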(event OnComponentBeginOverlap(Box)
  (params (OverlappedComponent :type Primitive%20Component%20Object%20Reference) (OtherActor :type Actor%20Object%20Reference) (OtherComp :type Primitive%20Component%20Object%20Reference) (OtherBodyIndex :type Integer) (bFromSweep :type Boolean) (SweepResult :type Hit%20Result%20Structure%20%28by%20ref%29))
  (bind _audio (Variables|Default|GetAudio))
  (bind _asfirst_person_character (Utilities|Casting|CastToFirstPersonCharacter OtherActor))
  (Variables|Default|SetPlayer%20HUD (Variables|/Game/Blueprints/FirstPersonCharacter.FirstPersonCharacter_C|GetPlayerHUD _asfirst_person_character))
  (Collision|SetCollisionEnabled (Variables|Default|GetBox) "NoCollision")
  (Audio|Components|Audio|SetSound (Variables|/Game/Blueprints/FirstPersonCharacter.FirstPersonCharacter_C|GetCharacterDialogueSoundComponent _asfirst_person_character) _audio)
  (Audio|Components|Audio|Play (Variables|/Game/Blueprints/FirstPersonCharacter.FirstPersonCharacter_C|GetCharacterDialogueSoundComponent _asfirst_person_character) 0.0)
  (Variables|Default|SetaudioLength (Variables|/Script/Engine.SoundBase|GetDuration _audio))
  (Default|UpdateSubtitleText (Variables|Default|GetPlayer%20HUD) (Variables|Default|GetCharacterName) (Variables|Default|GetCharacterDialogue))
  (Widget|SetVisibility (Variables|/Game/Blueprints/Widgets/BP_PlayerStatsWidget.BP_PlayerStatsWidget_C|GetSubtitleCanvas (Variables|Default|GetPlayer%20HUD)) "Visible")
  (Utilities|FlowControl|Delay (Variables|Default|GetaudioLength))
  (Widget|SetVisibility (Variables|/Game/Blueprints/Widgets/BP_PlayerStatsWidget.BP_PlayerStatsWidget_C|GetSubtitleCanvas (Variables|Default|GetPlayer%20HUD)) "Hidden")
  (Actor|DestroyActor))

(fn ConstructionScript
  (Components|Box|SetBoxExtent (Variables|Default|GetBox) (Variables|Default|GetboxExtentVector) true))