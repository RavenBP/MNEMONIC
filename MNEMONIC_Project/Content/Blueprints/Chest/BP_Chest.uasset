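; Openable chest actor that rewards the first-person character with currency and a spawned pickup.
; A trigger box toggles the chest's input and sets or clears the "Press E to Open Chest" prompt on the game mode's stat widget.
; OnInteraction opens it only once, playing the animation, disabling trigger collision, granting currency, then spawning the pickup at SpawnPoint after a short delay.
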(event OnComponentBeginOverlap(TriggerBox)
  (params (OverlappedComponent :type Primitive%20Component%20Object%20Reference) (OtherActor :type Actor%20Object%20Reference) (OtherComp :type Primitive%20Component%20Object%20Reference) (OtherBodyIndex :type Integer) (bFromSweep :type Boolean) (SweepResult :type Hit%20Result%20Structure%20%28by%20ref%29))
  (Utilities|Casting|CastToFirstPersonCharacter OtherActor)
  (Input|EnableInput (Game|GetPlayerController 0))
  (bind _ascustom_game_mode (Utilities|Casting|CastToCustomGameMode (Game|GetGameMode)))
  (Variables|/Game/Blueprints/Widgets/BP_PlayerStatsWidget.BP_PlayerStatsWidget_C|SetInteraction%20Text (Variables|/Game/Maps/CustomGameMode.CustomGameMode_C|GetPlayerStatWidget _ascustom_game_mode) "Press E to Open Chest"))

(event OnComponentEndOverlap(TriggerBox)
  (params (OverlappedComponent :type Primitive%20Component%20Object%20Reference) (OtherActor :type Actor%20Object%20Reference) (OtherComp :type Primitive%20Component%20Object%20Reference) (OtherBodyIndex :type Integer))
  (Utilities|Casting|CastToFirstPersonCharacter OtherActor)
  (Input|DisableInput (Game|GetPlayerController 0))
  (bind _ascustom_game_mode (Utilities|Casting|CastToCustomGameMode (Game|GetGameMode)))
  (Variables|/Game/Blueprints/Widgets/BP_PlayerStatsWidget.BP_PlayerStatsWidget_C|SetInteraction%20Text (Variables|/Game/Maps/CustomGameMode.CustomGameMode_C|GetPlayerStatWidget _ascustom_game_mode) ""))

(event EventBeginPlay)

(event Collision|EventActorBeginOverlap
  (params (OtherActor :type Actor%20Object%20Reference)))

(event EventTick
  (params (DeltaSeconds :type Float%20%28single-precision%29)))

(event EventOnInteraction
  (params (Player :type Character%20Object%20Reference))
  (Variables|Default|SetPlayerInteract Player)
  (if (Variables|Chest|GetChestOpened)
    (Development|PrintString "Chest Already Opened")
    (else
      (Variables|Chest|SetChestOpened true)
      (Components|Animation|PlayAnimation (Variables|Default|GetSkeletalMesh) "/Game/Animations/ChestV2/ChestOpening_Anim.ChestOpening_Anim" false)
      (Collision|SetCollisionEnabled (Variables|Default|GetTriggerBox) "NoCollision")
      (bind _asfirst_person_character (Utilities|Casting|CastToFirstPersonCharacter (Variables|Default|GetPlayerInteract)))
      (Default|CollectCurrency _asfirst_person_character (Variables|Chest|GetMind%20Guardian%20Currency))
      (Utilities|FlowControl|Delay 0.4)
      (Game|SpawnActorfromClass (Variables|Chest|GetPickUp) (Transformation|GetWorldTransform (Variables|Default|GetSpawnPoint)) "Undefined" 0 0))))

(fn ConstructionScript)