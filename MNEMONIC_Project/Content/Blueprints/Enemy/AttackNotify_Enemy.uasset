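; An enemy attack anim notify state that deals melee damage to the first-person player character during its window in the animation.
; Each tick it sphere-traces from a mesh socket along the owner's forward vector.
; A hit character takes damage once per window, tracked in a target list that clears when the notify begins.
; The character's first chaser hit also clears a flag and fires a one-time DamagedByChaser reaction.
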(fn ReceivedNotifyTick
  (params (MeshComp :type Skeletal%20Mesh%20Component%20Object%20Reference) (Animation :type Anim%20Sequence%20Base%20Object%20Reference) (FrameDeltaTime :type Float%20%28single-precision%29))
  (bind _socket (Variables|Default|GetSocket))
  (bind _hittargets (Variables|Default|GetHitTargets))
  (bind _returnvalue (Transformation|GetSocketLocation MeshComp _socket))
  (bind (_outhit _returnvalue_2) (Collision|SphereTraceForObjects MeshComp _returnvalue (+ _returnvalue (* (Transformation|GetActorForwardVector (Components|GetOwner MeshComp)) (Variables|Default|GetDistance))) (Variables|Default|GetRadius) (Variables|Default|GetObjectsToTrace) false 0 "None"))
  (if _returnvalue_2
    (bind _asfirst_person_character (Utilities|Casting|CastToFirstPersonCharacter (.hitactor _outhit)))
    (if (Utilities|Array|ContainsItem _hittargets _asfirst_person_character)
      _
      (else
        (Default|TookDamage _asfirst_person_character (Variables|Default|GetDamage))
        (if (Variables|/Game/Blueprints/Player/FirstPersonCharacter.FirstPersonCharacter_C|GetdamagedByChaserFirstTime _asfirst_person_character)
          (Variables|/Game/Blueprints/Player/FirstPersonCharacter.FirstPersonCharacter_C|SetdamagedByChaserFirstTime _asfirst_person_character false)
          (Default|DamagedbyChaser _asfirst_person_character))
        (Utilities|Array|Add _hittargets _asfirst_person_character)))
    (return false)))

(fn ReceivedNotifyBegin
  (params (MeshComp :type Skeletal%20Mesh%20Component%20Object%20Reference) (Animation :type Anim%20Sequence%20Base%20Object%20Reference) (TotalDuration :type Float%20%28single-precision%29))
  (Utilities|Array|Clear (Variables|Default|GetHitTargets))
  (return false))