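; BP_KnockBackComponent is an actor component that knocks back the Enemy that owns it.
; On BeginPlay it casts its owner to Enemy and caches that reference along with its AI controller, which the shown graphs do not use further.
; KnockBack applies a mass-dependent impulse through the enemy's CharacterMovement, combining the given direction scaled by Force with an upward VelocityZ boost, then prints a debug string.
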(event EventBeginPlay
  ;[1 1 1] Initialize variables
  (bind _asenemy (Utilities|Casting|CastToEnemy (Components|GetOwner)))
  (Variables|Default|SetEnemyRef _asenemy)
  (Variables|Default|SetAIControllerRef (AI|GetAIController (Variables|Default|GetEnemyRef))))

(event EventTick
  (params (DeltaSeconds :type Float%20%28single-precision%29)))

(fn KnockBack
  (params (Direction :type Vector))
  (Physics|AddImpulse (Variables|/Script/Engine.Character|GetCharacterMovement (Variables|Default|GetEnemyRef)) (+ (* Direction (Variables|Default|GetForce)) (* (Math|Vector|VectorUp) (Variables|Default|GetVelocityZ))) false)
  (Development|PrintString "KnockBack"))