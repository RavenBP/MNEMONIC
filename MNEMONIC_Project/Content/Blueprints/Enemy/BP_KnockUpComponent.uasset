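; Actor component that lets an owning Enemy be knocked into the air, pausing its AI while airborne.
; KnockUp triggers a Jump, using the jump velocity set at BeginPlay, and stops the AI controller's brain logic.
; While knocked up, Tick watches vertical velocity, temporarily overriding gravity scale once descent starts, then restoring it to 1 after a delay.
; AI logic restarts when vertical velocity reads exactly zero, which is treated as landing.
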(event EventBeginPlay
  ;[1 1 1] Initialize variables
  (bind _asenemy (Utilities|Casting|CastToEnemy (Components|GetOwner)))
  (bind _output_get (Variables|Default|SetEnemyRef _asenemy))
  (Variables|/Script/Engine.CharacterMovementComponent|SetJumpZVelocity (Variables|/Script/Engine.Character|GetCharacterMovement _output_get) (Variables|Default|GetVelocityZ))
  (Variables|Default|SetAIControllerRef (AI|GetAIController (Variables|Default|GetEnemyRef))))

(event EventTick
  (params (DeltaSeconds :type Float%20%28single-precision%29))
  (if (Variables|Default|GetKnockedUp)
    ;[1 1 1] Resume AI if knock back is done
    (if (== (.z (Transformation|GetVelocity (Variables|Default|GetEnemyRef))) 0.0)
      (CallFunction|ResumeAI))
    ;[1 1 1] If apex reached
    (if (< (.z (Transformation|GetVelocity (Variables|Default|GetEnemyRef))) 0.0)
      (Utilities|FlowControl|DoOnce false :!label _label
        (:Completed
          ;[1 1 1] Modify gravity
          (Variables|/Script/Engine.CharacterMovementComponent|SetGravityScale (Variables|/Script/Engine.Character|GetCharacterMovement (Variables|Default|GetEnemyRef)) (Variables|Default|GetGravity))
          (Utilities|FlowControl|Delay (Variables|Default|GetGravityTime))
          (Variables|/Script/Engine.CharacterMovementComponent|SetGravityScale (Variables|/Script/Engine.Character|GetCharacterMovement (Variables|Default|GetEnemyRef)) 1.0)))
      (else
        (goto _label Reset)))))

(fn KnockUp
  (Character|Jump (Variables|Default|GetEnemyRef))
  (AI|Logic|StopLogic (Variables|/Script/AIModule.AIController|GetBrainComponent (Variables|Default|GetAIControllerRef)) "Knock up")
  (Variables|Default|SetKnockedUp true))

(fn ResumeAI
  (AI|Logic|StartLogic (Variables|/Script/AIModule.AIController|GetBrainComponent (Variables|Default|GetAIControllerRef)))
  (Variables|Default|SetKnockedUp false))