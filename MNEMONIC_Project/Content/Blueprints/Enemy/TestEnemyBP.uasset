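; Enemy character Blueprint with a health bar, optional shield, target marking and knockback reactions, granting the player currency and speed stacks on death.
; Health events update the bar when unshielded, flag the chaser hit animation on damage, and knock back grounded shielded enemies.
; Player dash hits knock it back, while slide hits also knock up and remove the shield.
; A radius overlap runs a delay loop turning the bar toward the player; Tick rotates the visible marking.
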(event OnComponentBeginOverlap(HealthBarRadius)
  (params (OverlappedComponent :type Primitive%20Component%20Object%20Reference) (OtherActor :type Actor%20Object%20Reference) (OtherComp :type Primitive%20Component%20Object%20Reference) (OtherBodyIndex :type Integer) (bFromSweep :type Boolean) (SweepResult :type Hit%20Result%20Structure%20%28by%20ref%29))
  (Utilities|Casting|CastToFirstPersonCharacter OtherActor)
  (Variables|Default|SetisInHealthbarRadius true)
  (CallFunction|UpdateHealthbar))

(event OnComponentEndOverlap(HealthBarRadius)
  (params (OverlappedComponent :type Primitive%20Component%20Object%20Reference) (OtherActor :type Actor%20Object%20Reference) (OtherComp :type Primitive%20Component%20Object%20Reference) (OtherBodyIndex :type Integer))
  (Utilities|Casting|CastToFirstPersonCharacter OtherActor)
  (Variables|Default|SetisInHealthbarRadius false))

(event OnComponentHit(CapsuleComponent)
  (params (HitComponent :type Primitive%20Component%20Object%20Reference) (OtherActor :type Actor%20Object%20Reference) (OtherComp :type Primitive%20Component%20Object%20Reference) (NormalImpulse :type Vector :default "0, 0, 0") (Hit :type Hit%20Result%20Structure%20%28by%20ref%29))
  (bind _asfirst_person_character (Utilities|Casting|CastToFirstPersonCharacter OtherActor))
  (if (Variables|/Game/Blueprints/Player/FirstPersonCharacter.FirstPersonCharacter_C|GetdashAttackActive _asfirst_person_character)
    ;[1 1 1] Knock back if dashing
    (Default|KnockBack (Variables|Default|GetBP_KnockBackComponent) (Transformation|GetActorForwardVector (Game|Player|GetPlayerPawn 0)) true)
    (else
      ;[1 1 1] Knock up and Knock back if sliding
      (if (Utilities|Name|Equal(Name) (Variables|/Script/MNEMONIC_Project.IState|GetStateDisplayName (Variables|/Script/MNEMONIC_Project.StateManagerComponent|GetCurrentState (Variables|/Script/MNEMONIC_Project.MNEMONIC_ProjectCharacter|GetStateManager _asfirst_person_character))) "Slide")
        (Default|KnockUp (Variables|Default|GetBP_KnockUpComponent))
        (Default|KnockBack (Variables|Default|GetBP_KnockBackComponent) (Transformation|GetActorForwardVector (Game|Player|GetPlayerPawn 0)) false)
        (CallFunction|SetShield false)))))

(event Custom|healthEvent_Event_0
  (params (health :type Float%20%28single-precision%29) (addedHealth :type Float%20%28single-precision%29))
  (if (Variables|Shield|GethasShielded)
    _
    (else
      (bind _aswbp_enemy_health_bar (Utilities|Casting|CastToWBP_EnemyHealthBar (UserInterface|GetWidget (Variables|Default|GethealthBar))))
      (Progress|SetPercent (Variables|/Game/Blueprints/Widgets/WBP_EnemyHealthBar.WBP_EnemyHealthBar_C|GetProgressHealthBar _aswbp_enemy_health_bar) (/ health (.m_fmaxhealth (Variables|Default|Getstats))))))
  (if (< addedHealth 0.0)
    (bind _aschaser_anim_blueprint (Utilities|Casting|CastToChaserAnimBlueprint (Components|SkeletalMesh|GetAnimInstance (Variables|Character|GetMesh))))
    (Variables|/Game/Art/Animations/Enemies/Chaser/ChaserAnimBlueprint.ChaserAnimBlueprint_C|SetChaserHit _aschaser_anim_blueprint true)
    ;[1 1 1] Knock Back
    (if (Variables|Shield|GethasShielded)
      (if (AI|Components|NavMovement|IsMovingonGround (Variables|Character|GetCharacterMovement))
        (Default|KnockBack (Variables|Default|GetBP_KnockBackComponent) (Transformation|GetActorForwardVector (Game|Player|GetPlayerPawn 0)) false)))))

(event Custom|OnDeath
  ;[1 1 1] Death
  (if (not (Variables|Default|GetisDead))
    (bind _asfirst_person_character (Utilities|Casting|CastToFirstPersonCharacter (Game|Player|GetPlayerPawn 0)))
    (Default|CollectCurrency _asfirst_person_character (Variables|Default|GetMindGuardianCurrency))
    (Default|ModifySpeedStack _asfirst_person_character 1e+01)
    (Variables|Default|SetisDead true)
    (Actor|DestroyActor) ; NOTE: Need to play animation here before doing this once we have the animation
  ))

(event Custom|UpdateHealthbar
  (bind _healthbar (Variables|Default|GethealthBar))
  (if (Variables|Default|GetisInHealthbarRadius) :!label _label
    (Rendering|SetVisibility _healthbar true false)
    (Transformation|SetWorldRotation _healthbar (Math|Rotator|FindLookatRotation (Transformation|GetActorLocation) (Transformation|GetActorLocation (Game|Player|GetPlayerPawn 0))) false false)
    (Utilities|FlowControl|Delay 0.3)
    (goto _label)
    (else
      (Rendering|SetVisibility _healthbar false false))))

(event EventBeginPlay
  (bind _stats (Variables|Default|Getstats))
  (EventDispatchers|AssignHealthEvent (delegate Custom|healthEvent_Event_0))
  (Class|Enemy|AddHealth (.m_fmaxhealth (Variables|Default|Getstats)))
  (bind _aswbp_enemy_health_bar (Utilities|Casting|CastToWBP_EnemyHealthBar (UserInterface|GetWidget (Variables|Default|GethealthBar))))
  (Progress|SetPercent (Variables|/Game/Blueprints/Widgets/WBP_EnemyHealthBar.WBP_EnemyHealthBar_C|GetProgressHealthBar _aswbp_enemy_health_bar) (/ (.m_fmaxhealth _stats) (.m_fmaxhealth _stats)))
  (Utilities|FlowControl|Delay 1.0)
  (Transformation|AttachComponentToComponent (Variables|Default|GethealthBar) (Variables|Default|GetHealthbarTransform) "None" "SnapToTarget" "KeepRelative" "KeepRelative" true)
  (Rendering|SetVisibility (Variables|Default|GethealthBar) false false))

(event EventTick
  (params (DeltaSeconds :type Float%20%28single-precision%29))
  (CallFunction|SetRotationOfMarking))

(fn ConstructionScript
  (bind _markedtargetsensitivity (Variables|Marking|GetMarkedTargetSensitivity))
  (Transformation|SetWorldScale3D (Variables|Default|GetMarkedCollision) (Math|Vector|MakeVector _markedtargetsensitivity _markedtargetsensitivity _markedtargetsensitivity))
  (Rendering|SetVisibility (Variables|Default|GetMarking) false false)
  (Rendering|SetVisibility (Variables|Default|GetSphereShield) (Variables|Shield|GethasShielded) false))

(fn Mark
  (Rendering|SetVisibility (Variables|Default|GetMarking) true false))

(fn UnMark
  (Rendering|SetVisibility (Variables|Default|GetMarking) false false))

(fn SetRotationOfMarking
  (if (Rendering|IsVisible (Variables|Default|GetMarking))
    (Transformation|SetWorldRotation (Variables|Default|GetMarking) (Math|Rotator|MakeRotator 0.0 0.0 (Math|Trig|RadiansToDegrees (Class|KismetMathLibrary|VectorHeadingAngle (- (Transformation|GetActorLocation (Game|Player|GetPlayerPawn 0)) (Transformation|GetActorLocation))))) false false)))

(fn SetShield
  (params (value :type Boolean))
  (bind _output_get (Variables|Shield|SethasShielded value))
  (Rendering|SetVisibility (Variables|Default|GetSphereShield) _output_get false))