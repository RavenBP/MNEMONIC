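; Gate actor that opens a portal as the player nears and, on contact, shows a card screen tied to the next level.
; A sphere of configurable radius triggers a timeline that scales the portal mesh along X.
; Touching the mesh clears existing widgets, fills three cards from random class defaults in separate pools, passes the next level name, pauses the game and destroys the gate.
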(event OnComponentBeginOverlap(StaticMesh)
  (params (OverlappedComponent :type Primitive%20Component%20Object%20Reference) (OtherActor :type Actor%20Object%20Reference) (OtherComp :type Primitive%20Component%20Object%20Reference) (OtherBodyIndex :type Integer) (bFromSweep :type Boolean) (SweepResult :type Hit%20Result%20Structure%20%28by%20ref%29))
  (bind _returnvalue (Game|GetPlayerController 0))
  (Utilities|Casting|CastToFirstPersonCharacter OtherActor)
  (Viewport|RemoveAllWidgets)
  (bind _returnvalue_2 (UserInterface|CreateWidget "/Game/Blueprints/Gate/Wd_Gate.Wd_Gate_C"))
  (CallFunction|SetWidgetCards _returnvalue_2)
  (Default|UpdateWidget _returnvalue_2)
  (UserInterface|Viewport|AddtoViewport _returnvalue_2 0)
  (Game|SetGamePaused true)
  (Input|SetInputModeGameandUI _returnvalue _returnvalue_2 "DoNotLock" false)
  (Variables|/Script/Engine.PlayerController|SetbShowMouseCursor _returnvalue true)
  (Actor|DestroyActor))

(event OnComponentBeginOverlap(Sphere)
  (params (OverlappedComponent :type Primitive%20Component%20Object%20Reference) (OtherActor :type Actor%20Object%20Reference) (OtherComp :type Primitive%20Component%20Object%20Reference) (OtherBodyIndex :type Integer) (bFromSweep :type Boolean) (SweepResult :type Hit%20Result%20Structure%20%28by%20ref%29))
  (bind _staticmesh (Variables|Default|GetStaticMesh))
  (bind _returnvalue (Transformation|GetWorldScale _staticmesh))
  (Utilities|Casting|CastToFirstPersonCharacter OtherActor)
  (Variables|Default|SetplayerEnteredRadius true)
  (bind _xscale (Timeline|ScalePortal Play)
    (:Update
      (Transformation|SetWorldScale3D _staticmesh (Math|Vector|MakeVector _xscale (.y _returnvalue) (.z _returnvalue))))))

(fn ConstructionScript
  (Components|Sphere|SetSphereRadius (Variables|Default|GetSphere) (Variables|Default|GetgateActivationRadius) true))

(fn SetWidgetCards
  (params (Widget :type Wd%20Gate%20Object%20Reference))
  (CallFunction|SetCardfromPool (Variables|/Game/Blueprints/Gate/Wd_Gate.Wd_Gate_C|GetCard1 Widget) (Variables|Gate|GetCardsPool1))
  (CallFunction|SetCardfromPool (Variables|/Game/Blueprints/Gate/Wd_Gate.Wd_Gate_C|GetCard2 Widget) (Variables|Gate|GetCardsPool2))
  (CallFunction|SetCardfromPool (Variables|/Game/Blueprints/Gate/Wd_Gate.Wd_Gate_C|GetCard3 Widget) (Variables|Gate|GetCardsPool3))
  (Variables|/Game/Blueprints/Gate/Wd_Gate.Wd_Gate_C|SetNextLevelName Widget (Variables|Gate|GetNextLevel%20Name)))

(fn SetCardfromPool
  (params (card :type Struct%20Card%20Structure%20%28by%20ref%29) (CardPool :type Array%20of%20DA%20Card%20Base%20Class%20References))
  (|SetBy-RefVar card (Utilities|GetClassDefaults (Utilities|Array|Get(acopy) CardPool (Math|Random|RandomInteger (Utilities|Array|Length CardPool))))))