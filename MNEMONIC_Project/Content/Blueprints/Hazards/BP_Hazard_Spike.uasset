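; Spike hazard that damages the FirstPersonCharacter while it overlaps the hazard's Box.
; Begin overlap stores the player reference, applies damage immediately and resets the timer, while end overlap clears the reference and flag.
; Tick accumulates delta time during overlap and reapplies damage each time the timer reaches TickRate.
; Damage passes DamageToPlayer straight into AddToCurrentHealth, so its sign determines whether health drops.
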(event OnComponentBeginOverlap(Box)
  (params (OverlappedComponent :type Primitive%20Component%20Object%20Reference) (OtherActor :type Actor%20Object%20Reference) (OtherComp :type Primitive%20Component%20Object%20Reference) (OtherBodyIndex :type Integer) (bFromSweep :type Boolean) (SweepResult :type Hit%20Result%20Structure%20%28by%20ref%29))
  (bind _asfirst_person_character (Utilities|Casting|CastToFirstPersonCharacter OtherActor))
  (Variables|Default|SetPlayerRef _asfirst_person_character)
  (Variables|Default|SetisOverlappingWithPlayer true)
  ;[1 1 1] Player take damage
  (Class|MNEMONICProjectCharacter|AddtoCurrentHealth (Variables|Default|GetPlayerRef) (Variables|Hazard|GetDamageToPlayer))
  (Variables|Default|SetTimer 0.0))

(event OnComponentEndOverlap(Box)
  (params (OverlappedComponent :type Primitive%20Component%20Object%20Reference) (OtherActor :type Actor%20Object%20Reference) (OtherComp :type Primitive%20Component%20Object%20Reference) (OtherBodyIndex :type Integer))
  (Utilities|Casting|CastToFirstPersonCharacter OtherActor)
  (Variables|Default|SetPlayerRef 0)
  (Variables|Default|SetisOverlappingWithPlayer false))

(event EventTick
  (params (DeltaSeconds :type Float%20%28single-precision%29))
  (if (Variables|Default|GetisOverlappingWithPlayer)
    ;[1 1 1] timer Update
    (bind _output_get (Variables|Default|SetTimer (+ (Variables|Default|GetTimer) DeltaSeconds)))
    ;[1 1 1] timer > tickrate
    (if (>= _output_get (Variables|Hazard|GetTickRate))
      ;[1 1 1] Player take damage
      (Class|MNEMONICProjectCharacter|AddtoCurrentHealth (Variables|Default|GetPlayerRef) (Variables|Hazard|GetDamageToPlayer))
      (Variables|Default|SetTimer 0.0))))

(fn ConstructionScript)