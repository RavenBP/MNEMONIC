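; BP_TutorialArena is a trigger volume that spawns a single enemy the first time the player enters the tutorial arena.
; When the first-person character overlaps the box, it spawns a TestEnemyBP running BT_Grunt at a random chaser spawn location, guarded by an entered-once flag.
; It then reattaches the enemy's health bar to its transform component, and the construction script sizes the box from an editable extent.
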(event OnComponentBeginOverlap(Box)
  (params (OverlappedComponent :type Primitive%20Component%20Object%20Reference) (OtherActor :type Actor%20Object%20Reference) (OtherComp :type Primitive%20Component%20Object%20Reference) (OtherBodyIndex :type Integer) (bFromSweep :type Boolean) (SweepResult :type Hit%20Result%20Structure%20%28by%20ref%29))
  (Utilities|Casting|CastToFirstPersonCharacter OtherActor)
  (CallFunction|PlayerEnteredArena))

(event Custom|PlayerEnteredArena
  (if (Variables|Default|GetplayerAlreadyEnteredArena)
    (Development|PrintString "Player Already entered")
    (else
      (Variables|Default|SetplayerAlreadyEnteredArena true)
      (bind _returnvalue (AI|SpawnAIFromClass "/Game/Blueprints/Enemy/TestEnemyBP.TestEnemyBP_C" "/Game/Blueprints/Enemy/BT_Grunt.BT_Grunt" (.location (.OutItem (Utilities|Array|Random (Variables|Default|GetChaserSpawnLocation)))) "0, 0, 0" false 0))
      (bind _output_get (Variables|Default|SetSpawnedEnemy _returnvalue))
      (bind _astest_enemy_bp (Utilities|Casting|CastToTestEnemyBP _output_get))
      (Transformation|AttachComponentToComponent (Variables|/Script/MNEMONIC_Project.Enemy|GethealthBar _astest_enemy_bp) (Variables|/Game/Blueprints/Enemy/TestEnemyBP.TestEnemyBP_C|GetHealthbarTransform _astest_enemy_bp) "None" "KeepRelative" "KeepRelative" "KeepRelative" true)
      (Development|PrintString "Hello"))))

(fn ConstructionScript
  (Components|Box|SetBoxExtent (Variables|Default|GetBox) (Variables|Default|GetBoxExtent) true))