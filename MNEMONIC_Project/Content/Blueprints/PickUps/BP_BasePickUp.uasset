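; Base pickup actor that shows an item info widget and grants the first-person player new stats when collected.
; BeginPlay caches the player and fills the widget from the PickUp data.
; Collider overlap toggles Pickable and input, while Tick syncs widget visibility to that flag and prints a debug stats string.
; Pressing Interact while in range plays the pickup animation and sound, applies the stats, then destroys the actor.
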(event OnComponentBeginOverlap(StatsColliderMessage)
  (params (OverlappedComponent :type Primitive%20Component%20Object%20Reference) (OtherActor :type Actor%20Object%20Reference) (OtherComp :type Primitive%20Component%20Object%20Reference) (OtherBodyIndex :type Integer) (bFromSweep :type Boolean) (SweepResult :type Hit%20Result%20Structure%20%28by%20ref%29))
  ;[1 1 1] Overlapping - Debug Message creation
  (Utilities|Casting|CastToFirstPersonCharacter OtherActor)
  (Variables|Default|SetPickable true)
  (Input|EnableInput (Game|GetPlayerController 0)))

(event OnComponentEndOverlap(StatsColliderMessage)
  (params (OverlappedComponent :type Primitive%20Component%20Object%20Reference) (OtherActor :type Actor%20Object%20Reference) (OtherComp :type Primitive%20Component%20Object%20Reference) (OtherBodyIndex :type Integer))
  ;[1 1 1] End Overlapping
  (Utilities|Casting|CastToFirstPersonCharacter OtherActor)
  (Variables|Default|SetPickable false)
  (Input|DisableInput (Game|GetPlayerController 0)))

(event EventBeginPlay
  ;[1 1 1] Get PlayerRef
  (bind _asfirst_person_character (Utilities|Casting|CastToFirstPersonCharacter (Game|Player|GetPlayerPawn 0)))
  (Variables|Default|SetPlayerRef _asfirst_person_character)
  ;[1 1 1] Set widget
  (CallFunction|SetWidget))

(event EventTick
  (params (DeltaSeconds :type Float%20%28single-precision%29))
  (bind _pickable (Variables|Default|GetPickable))
  ;[1 1 1] Debug Message (This can probably be removed from event tick (do 2 events for when the player is InRange and !InRange))
  (if _pickable
    (Development|PrintString (Variables|Default|GetPickUpStats) true true "(R=0.000000,G=0.660000,B=1.000000,A=1.000000)" 0.0))
  (Rendering|SetVisibility (Variables|PickUp|GetWidget) _pickable false))

(event Input|ActionEvents|InputActionInteract
  (params (Key :type Key%20Structure))
  ;[1 1 1] Player Pick up the Pickup
  (:Pressed
    (if (Variables|Default|GetPickable)
      (Default|PickUpAnimation (Variables|Default|GetPlayerRef))
      ;[1 1 1] Modify Player Stats
      (Default|AddNewStats (Variables|Default|GetPlayerRef) (.pickupstats (Variables|PickUp|GetPickUp)))
      (Audio|PlaySound2D "/Game/Audio/Player/Pickup.Pickup" 1.0 1.0 0.0 0 0)
      (Actor|DestroyActor))))

(fn ConstructionScript)

(fn NewMessageStat
  (params (Stat :type Float%20%28single-precision%29) (StatName :type String))
  (if (!= Stat 0.0)
    (Variables|Default|SetPickUpStats (Utilities|String|Append (Variables|Default|GetPickUpStats) (Utilities|String|Append (Utilities|String|Append StatName (Utilities|String|ToString(Float) Stat)) "  || ")))))

(fn SetWidget
  (bind _asui_pickup_window (Utilities|Casting|CastToUI_PickupWindow (UserInterface|GetWidget (Variables|PickUp|GetWidget))))
  ;[1 1 1] Name
  (Rendering|Components|TextRender|SetText (Variables|/Game/Blueprints/PickUps/UI_PickupWindow.UI_PickupWindow_C|GetItemNameText _asui_pickup_window) (Utilities|Text|ToText(Name) (.name (Variables|PickUp|GetPickUp))))
  ;[1 1 1] rarity
  (Rendering|Components|TextRender|SetText (Variables|/Game/Blueprints/PickUps/UI_PickupWindow.UI_PickupWindow_C|GetRarityText _asui_pickup_window) (Utilities|Text|ToText(String) (Utilities|String|EnumtoString (.rarity (Variables|PickUp|GetPickUp)))))
  ;[1 1 1] Description
  (Rendering|Components|TextRender|SetText (Variables|/Game/Blueprints/PickUps/UI_PickupWindow.UI_PickupWindow_C|GetDescriptionText _asui_pickup_window) (Utilities|Text|ToText(String) (.description (Variables|PickUp|GetPickUp))))
  ;[1 1 1] Image
  (Appearance|SetBrushfromTexture (Variables|/Game/Blueprints/PickUps/UI_PickupWindow.UI_PickupWindow_C|GetItemImage _asui_pickup_window) (.image (Variables|PickUp|GetPickUp)) true)
  ;[1 1 1] Effect text
  (Rendering|Components|TextRender|SetText (Variables|/Game/Blueprints/PickUps/UI_PickupWindow.UI_PickupWindow_C|GetEffectText _asui_pickup_window) (Utilities|Text|ToText(String) (.statschangetext (Variables|PickUp|GetPickUp)))))