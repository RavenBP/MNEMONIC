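; BP_PlayerAttack is a player state in which the first-person character attacks a marked enemy.
; On enter it casts the player reference to FirstPersonCharacter, caches it and calls AttackMarkedEnemy.
; Each tick it pops itself from the StateManager once IsAttackingEnemyMarked is false.
; Primary weapon and movement input events are overridden with empty bodies, so those inputs do nothing during the attack.
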(event EventPressMoveRight
  (params (value :type Float%20%28single-precision%29)))

(event EventTickState
  (if (not (Variables|/Game/Blueprints/Player/FirstPersonCharacter.FirstPersonCharacter_C|GetIsAttackingEnemyMarked (Variables|Default|GetfirstPersonCref)))
    (Class|StateManagerComponent|PopState (Variables|/Script/MNEMONIC_Project.MNEMONIC_ProjectCharacter|GetStateManager (Variables|Default|GetPlayerRef)))))

(event EventOnEnterState
  (params (StateOwner :type Actor%20Object%20Reference))
  (|CallParentFunction StateOwner)
  (bind _asfirst_person_character (Utilities|Casting|CastToFirstPersonCharacter (Variables|Default|GetPlayerRef)))
  (bind _output_get (Variables|Default|SetfirstPersonCref _asfirst_person_character))
  (Default|AttackMarkedEnemy _output_get))

(event EventPressPrimaryWeapon
  (params (value :type Boolean)))

(event EventPressMoveForward
  (params (value :type Float%20%28single-precision%29)))