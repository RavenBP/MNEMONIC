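; Player idle state for the first-person character's state machine, handling input while idle.
; On enter it caches the player as a FirstPersonCharacter reference.
; Primary weapon input pushes the HyperSlice state when an enemy is marked, otherwise it uses the parent behaviour.
; Look and turn input pass to the parent only while the character is not targeting.
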(event EventPressPrimaryWeapon
  (params (value :type Boolean))
  (if value
    (Utilities|IsValid (Variables|/Game/Blueprints/Player/FirstPersonCharacter.FirstPersonCharacter_C|GetEnemyMarked (Variables|Default|GetfpcharacterRef))
      (:Is%20Valid
        (Class|StateManagerComponent|PushStatebyKey (Variables|/Script/MNEMONIC_Project.MNEMONIC_ProjectCharacter|GetStateManager (Variables|Default|GetPlayerRef)) "HyperSlice"))
      (:Is%20Not%20Valid
        (|CallParentFunction value)))))

(event EventOnEnterState
  (params (StateOwner :type Actor%20Object%20Reference))
  (|CallParentFunction StateOwner)
  (bind _asfirst_person_character (Utilities|Casting|CastToFirstPersonCharacter (Variables|Default|GetPlayerRef)))
  (Variables|Default|SetfpcharacterRef _asfirst_person_character))

(event EventPressLookUp
  (params (value :type Float%20%28single-precision%29))
  (if (not (Variables|/Game/Blueprints/Player/FirstPersonCharacter.FirstPersonCharacter_C|GetIsTargetting (Variables|Default|GetfpcharacterRef)))
    (|CallParentFunction value)))

(event EventPressTurn
  (params (value :type Float%20%28single-precision%29))
  (if (not (Variables|/Game/Blueprints/Player/FirstPersonCharacter.FirstPersonCharacter_C|GetIsTargetting (Variables|Default|GetfpcharacterRef)))
    (|CallParentFunction value)))