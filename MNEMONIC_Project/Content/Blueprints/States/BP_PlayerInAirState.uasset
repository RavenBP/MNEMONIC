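; Player state for being airborne in a first-person character's state machine, handling primary attacks in mid-air.
; A primary press pushes the HyperSlice state if an enemy is marked; otherwise it runs the parent attack once the attack montage has stopped.
; Each air attack changes gravity scale, with the first also zeroing velocity, then calls the character's DefaultGravity.
; Tick prints the current gravity scale for debugging.
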(event EventPressPrimaryWeapon
  (params (value :type Boolean))
  (if value
    (Utilities|IsValid (Variables|/Game/Blueprints/Player/FirstPersonCharacter.FirstPersonCharacter_C|GetEnemyMarked (Variables|Default|GetFPcharacterRef))
      (:Is%20Valid
        (Class|StateManagerComponent|PushStatebyKey (Variables|/Script/MNEMONIC_Project.MNEMONIC_ProjectCharacter|GetStateManager (Variables|Default|GetPlayerRef)) "HyperSlice"))
      (:Is%20Not%20Valid
        (if (Class|AnimInstance|MontageGetIsStopped (Components|SkeletalMesh|GetAnimInstance (Variables|/Script/MNEMONIC_Project.MNEMONIC_ProjectCharacter|GetMesh1P (Variables|Default|GetFPcharacterRef))) "/Game/Animations/Player/Misc/PlayerAttack_Animation_Montage.PlayerAttack_Animation_Montage")
          (|CallParentFunction value)
          ;[1 1 1] Reduce gravity if attacks
          (bind _result (Math|Integer|IncrementInt (Variables|Default|GetCountAttacks))
            (:%20%20
              (if (== _result 1)
                (CallFunction|SetGravity (Variables|Default|GetGravityScaleFirstAttack) true)
                (else
                  (CallFunction|SetGravity (Variables|Default|GetGravityScaleAfterFirstAttack) false)))
              (Default|DefaultGravity (Variables|Default|GetFPcharacterRef)))))))))

(event EventOnEnterState
  (params (StateOwner :type Actor%20Object%20Reference))
  (|CallParentFunction StateOwner)
  (bind _asfirst_person_character (Utilities|Casting|CastToFirstPersonCharacter (Variables|Default|GetPlayerRef)))
  (Variables|Default|SetFPcharacterRef _asfirst_person_character)
  (Variables|Default|SetCountAttacks 0))

(event EventTickState
  (|CallParentFunction)
  (Development|PrintString 0 (Utilities|String|ToString(Float) (Variables|/Script/Engine.CharacterMovementComponent|GetGravityScale (Variables|/Script/Engine.Character|GetCharacterMovement (Variables|Default|GetFPcharacterRef)))) true true "(R=1.000000,G=0.000000,B=0.578436,A=1.000000)" 0.0))

(fn SetGravity
  (params (GravityScale :type Float%20%28single-precision%29) (isFirstTime :type Boolean))
  (bind _playerref (Variables|Default|GetPlayerRef))
  (bind _charactermovement (Variables|/Script/Engine.Character|GetCharacterMovement _playerref))
  (Variables|/Script/Engine.CharacterMovementComponent|SetGravityScale _charactermovement GravityScale)
  (if isFirstTime
    (Variables|/Script/Engine.MovementComponent|SetVelocity _charactermovement (Math|Vector|MakeVector 0.0 0.0 0.0))))