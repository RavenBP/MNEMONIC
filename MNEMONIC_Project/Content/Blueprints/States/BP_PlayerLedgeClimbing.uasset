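; BP_PlayerLedgeClimbing is a player state that runs while the first-person character climbs a ledge.
; On entry it casts the player reference to FirstPersonCharacter and calls LedgeClimb on it.
; Each tick it checks the character's IsLedgeClimbing flag and pops itself off the StateManager stack once the climb ends.
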(event EventOnEnterState
  (params (StateOwner :type Actor%20Object%20Reference))
  (|CallParentFunction StateOwner)
  (bind _output_get (Variables|Default|SetcharacterRef (.AsFirst%20Person%20Character (Utilities|Casting|CastToFirstPersonCharacter (Variables|Default|GetPlayerRef)))))
  (Default|LedgeClimb _output_get))

(event EventTickState
  (bind _characterref (Variables|Default|GetcharacterRef))
  (|CallParentFunction)
  (if (not (Variables|/Game/Blueprints/Player/FirstPersonCharacter.FirstPersonCharacter_C|GetisLedgeClimbing _characterref))
    (Class|StateManagerComponent|PopState (Variables|/Script/MNEMONIC_Project.MNEMONIC_ProjectCharacter|GetStateManager _characterref))))