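; Player state Blueprint for sliding, layered on a parent state's enter, tick and input handlers.
; On entry it casts the player reference to FirstPersonCharacter and stores it.
; Look and turn input pass to the parent only while the character is not targeting, and primary weapon input is overridden to do nothing.
; Each tick it prints the speed from the movement component's last update velocity.
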(event EventPressPrimaryWeapon
  (params (value :type Boolean)))

(event EventOnEnterState
  (params (StateOwner :type Actor%20Object%20Reference))
  (|CallParentFunction StateOwner)
  (bind _asfirst_person_character (Utilities|Casting|CastToFirstPersonCharacter (Variables|Default|GetPlayerRef)))
  (Variables|Default|SetFPcharacterRef _asfirst_person_character))

(event EventPressLookUp
  (params (value :type Float%20%28single-precision%29))
  (if (not (Variables|/Game/Blueprints/Player/FirstPersonCharacter.FirstPersonCharacter_C|GetIsTargetting (Variables|Default|GetfpcharacterRef)))
    (|CallParentFunction value)))

(event EventPressTurn
  (params (value :type Float%20%28single-precision%29))
  (if (not (Variables|/Game/Blueprints/Player/FirstPersonCharacter.FirstPersonCharacter_C|GetIsTargetting (Variables|Default|GetfpcharacterRef)))
    (|CallParentFunction value)))

(event EventTickState
  (|CallParentFunction)
  (Development|PrintString 0 (Utilities|String|ToString(Float) (Math|Vector|VectorLength (Pawn|Components|CharacterMovement|GetLastUpdateVelocity (Variables|/Script/Engine.Character|GetCharacterMovement (Variables|Default|GetPlayerRef))))) true true "(R=0.000000,G=0.660000,B=1.000000,A=1.000000)" 0.0))