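; Test enemy Blueprint that shows its health on a widget bar and reacts to damage.
; On BeginPlay it binds a health event and adds its maximum health from Stats.
; Each health event sets the WBP_EnemyHealthBar progress to the current health fraction.
; When the added health is negative, it also sets the HitAnim flag on TestEnemyAnimBP.
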(event Custom|healthEvent_Event_0
  (params (health :type Float%20%28single-precision%29) (addedHealth :type Float%20%28single-precision%29))
  (bind _aswbp_enemy_health_bar (Utilities|Casting|CastToWBP_EnemyHealthBar (UserInterface|GetWidget (Variables|Default|GetWidget))))
  (Progress|SetPercent (Variables|/Game/Blueprints/WBP_EnemyHealthBar.WBP_EnemyHealthBar_C|GetProgressHealthBar _aswbp_enemy_health_bar) (/ health (.m_fmaxhealth (Variables|Default|Getstats))))
  (if (< addedHealth 0.0)
    (bind _astest_enemy_anim_bp (Utilities|Casting|CastToTestEnemyAnimBP (Components|SkeletalMesh|GetAnimInstance (Variables|Character|GetMesh))))
    (Variables|/Game/Models/TestEnemy/TestEnemyAnimBP.TestEnemyAnimBP_C|SetHitAnim _astest_enemy_anim_bp true)))

(event EventBeginPlay
  (EventDispatchers|AssignHealthEvent (delegate Custom|healthEvent_Event_0))
  (Class|Enemy|AddHealth (.m_fmaxhealth (Variables|Default|Getstats))))

(fn ConstructionScript)