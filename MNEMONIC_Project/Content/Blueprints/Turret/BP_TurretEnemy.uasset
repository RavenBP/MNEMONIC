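; Turret enemy that turns to face a sensed player and fires damage-carrying projectiles alongside an attack montage, gated by a cooldown between shots.
; Health events update a widget health bar, flag the hit animation on damage, and on death award Mind Guardian currency to the player before destroying the turret.
; An overlap radius shows the health bar, re-aiming it at the player through a delay loop until the player leaves.
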(event OnSeePawn(PawnSensing)
  (params (Pawn :type Pawn%20Object%20Reference))
  (bind _asfirst_person_character (Utilities|Casting|CastToFirstPersonCharacter Pawn))
  (Utilities|FlowControl|Sequence
    (:then_0
      (Transformation|SetActorRotation (Math|Rotator|FindLookatRotation (Transformation|GetActorLocation) (Transformation|GetActorLocation _asfirst_person_character))))
    (:then_1
      (if (Variables|Default|GetspawnProjectile)
        (Animation|Montage|PlayMontage (Variables|Character|GetMesh) "/Game/Animations/Turret/Turret_Attack_Anim_Montage.Turret_Attack_Anim_Montage" ; TEMP FOR NOW
          (:then
            (bind _returnvalue (Game|SpawnActorfromClass "/Game/Blueprints/Turret/BP_EnemyProjectile.BP_EnemyProjectile_C" (Transformation|GetWorldTransform (Variables|Default|GetProjectileSpawnLocation)) "Undefined" 0 0))
            (Variables|/Game/Blueprints/Turret/BP_EnemyProjectile.BP_EnemyProjectile_C|SetprojectileDamage _returnvalue (Variables|Default|Getattack))
            (Variables|Default|SetspawnProjectile false)
            (Utilities|FlowControl|Delay (Variables|Default|GettimeBetweenShots))
            (Variables|Default|SetspawnProjectile true)))))))

(event OnComponentBeginOverlap(HealthBarRadius)
  (params (OverlappedComponent :type Primitive%20Component%20Object%20Reference) (OtherActor :type Actor%20Object%20Reference) (OtherComp :type Primitive%20Component%20Object%20Reference) (OtherBodyIndex :type Integer) (bFromSweep :type Boolean) (SweepResult :type Hit%20Result%20Structure%20%28by%20ref%29))
  (Utilities|Casting|CastToFirstPersonCharacter OtherActor)
  (Variables|Default|SetisInHealthBarRadius true)
  (CallFunction|UpdateHealthBar))

(event OnComponentEndOverlap(HealthBarRadius)
  (params (OverlappedComponent :type Primitive%20Component%20Object%20Reference) (OtherActor :type Actor%20Object%20Reference) (OtherComp :type Primitive%20Component%20Object%20Reference) (OtherBodyIndex :type Integer))
  (Utilities|Casting|CastToFirstPersonCharacter OtherActor)
  (Variables|Default|SetisInHealthBarRadius false))

(event Custom|healthEvent_Event_0
  (params (health :type Float%20%28single-precision%29) (addedHealth :type Float%20%28single-precision%29))
  (bind _aswbp_enemy_health_bar (Utilities|Casting|CastToWBP_EnemyHealthBar (UserInterface|GetWidget (Variables|Default|GethealthBar))))
  (Progress|SetPercent (Variables|/Game/Blueprints/Widgets/WBP_EnemyHealthBar.WBP_EnemyHealthBar_C|GetProgressHealthBar _aswbp_enemy_health_bar) (/ health (.m_fmaxhealth (Variables|Default|Getstats))))
  (if (< addedHealth 0.0)
    (bind _asturret_anim_blueprint (Utilities|Casting|CastToTurretAnimBlueprint (Components|SkeletalMesh|GetAnimInstance (Variables|Character|GetMesh))))
    (Variables|/Game/Blueprints/Turret/TurretAnimBlueprint.TurretAnimBlueprint_C|SetturretHit _asturret_anim_blueprint true)
    (bind _returnvalue (Class|Enemy|GetCurrentHealth))
    (if (<= _returnvalue 0.0)
      (CallFunction|OnDeath))))

(event Custom|OnDeath
  (bind _asfirst_person_character (Utilities|Casting|CastToFirstPersonCharacter (Game|Player|GetPlayerPawn 0)))
  (Default|CollectCurrency _asfirst_person_character (Variables|Default|GetmindGuardianCurrency))
  (Actor|DestroyActor))

(event Custom|UpdateHealthBar
  (bind _healthbar (Variables|Default|GethealthBar))
  (if (Variables|Default|GetisInHealthBarRadius) :!label _label
    (Rendering|SetVisibility _healthbar true false)
    (Transformation|SetWorldRotation _healthbar (Math|Rotator|FindLookatRotation (Transformation|GetActorLocation) (Transformation|GetActorLocation (Game|Player|GetPlayerPawn 0))) false false)
    (Utilities|FlowControl|Delay 0.3)
    (goto _label)
    (else
      (Rendering|SetVisibility _healthbar false false))))

(event EventBeginPlay
  (EventDispatchers|AssignHealthEvent (delegate Custom|healthEvent_Event_0))
  (Class|Enemy|AddHealth (.m_fmaxhealth (Variables|Default|Getstats)))
  (Utilities|FlowControl|Delay 1.0)
  (Transformation|AttachComponentToComponent (Variables|Default|GethealthBar) (Variables|Default|GetHealthBarTransform) "None" "SnapToTarget" "KeepRelative" "KeepRelative" true)
  (Rendering|SetVisibility (Variables|Default|GethealthBar) false false))

(fn ConstructionScript)